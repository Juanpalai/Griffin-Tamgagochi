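; Game mode for a Tamagotchi-style pet game that runs turn-based battles between the pet and a spawned enemy.
; Battle start switches the pet's UI, state and camera, then ChooseTurn alternates combatants through a shift counter, checking health for victory or defeat first.
; Status messages play through the pet's animated dialogue widget.
; It also saves and loads pet stats and derives time of day from the system clock; last-session calculation is an empty stub.
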(event `self.ReceiveBeginPlay`
  (bind _returnvalue (`GameplayStatics.GetActorOfClass` "/Game/Platzi/Core/Creature/Ped/BP_TamgochiPet.BP_TamgochiPet_C"))
  (set `self.refPet` _returnvalue)
  (set `PlayerController.bShowMouseCursor` true (`GameplayStatics.GetPlayerController` 0)))

(event `starBattle`
  (bind _refpet (`self.refPet`))
  (bind _output_get (set `self.battleMessege` "A wild dragon appeared  "))
  (`self.ShowMessege` _output_get)
  ;[1 1 1] Change Menu
  (`/Game/Platzi/Core/Creature/Ped/BP_TamgochiPet.ShowButtons` (`self.refPet`))
  (`/Game/Platzi/Core/Creature/Ped/BP_TamgochiPet.changeState` (`self.refPet`) "NewEnumerator1")
  (`self.spawnEnemy`)
  (`/Game/Platzi/Core/Creature/Ped/BP_TamgochiPet.CameraBattle` _refpet)
  (`KismetSystemLibrary.Delay` 2.0)
  (`SceneComponent.K2_SetRelativeRotation` (`/Game/Platzi/Core/Creature/BP_Tamagochibase.SkeletalMesh` _refpet) (struct :`Yaw` 45.0) false false)
  ;[1 1 1] Select Combat Turn
  (`self.chooseTurn`))

(event `EndBattle`
  (`/Game/Platzi/Core/Creature/Ped/BP_TamgochiPet.HideAtackbuttons` (`self.refPet`))
  (`/Game/Platzi/Core/Creature/Ped/BP_TamgochiPet.changeState` (`self.refPet`) "NewEnumerator0"))

(event `ShowMessege`
  (params (InText :type Text))
  (bind _refwidget (`/Game/Platzi/Core/Creature/Ped/BP_TamgochiPet.RefWidget` (`self.refPet`)))
  (bind _refwidget_2 (`/Game/Platzi/Core/Creature/Ped/BP_TamgochiPet.RefWidget` (`self.refPet`)))
  (`KismetSystemLibrary.Delay` 0.2)
  (`UserWidget.PlayAnimation` _refwidget_2 (`/Game/Platzi/UI/WBP_Main.ShowDialogue` _refwidget_2) 0.0 1 "Forward" 1.0 false)
  (`TextBlock.SetText` (`/Game/Platzi/UI/WBP_Main.TextActions` _refwidget_2) InText)
  (`KismetSystemLibrary.Delay` 2.0)
  (`UserWidget.PlayAnimation` _refwidget (`/Game/Platzi/UI/WBP_Main.ShowDialogue` _refwidget) 0.0 1 "Reverse" 1.0 false))

(event `RatateStarPosition`
  (bind _refpet (`self.refPet`))
  (`KismetSystemLibrary.Delay` 1.0)
  (`/Game/Platzi/Core/Creature/Ped/BP_TamgochiPet.Fadein` _refpet)
  (`SceneComponent.K2_SetRelativeRotation` (`/Game/Platzi/Core/Creature/BP_Tamagochibase.SkeletalMesh` _refpet) (struct :`Yaw` -90.0) false false))

(fn `calculateLastSession`
  (locals (NewLocalVar_0 :type "DateTime Structure"))
  ;[1 1 1] Not available in UE5 early access
)

(fn `chechVictory`
  (bind _refenemy (`self.refEnemy`)
    (:`then`
      (if (<= (`/Game/Platzi/Core/Creature/BP_Tamagochibase.Health` _refenemy) 0.0)
        (set `self.battleStatus ` "NewEnumerator0" :!label _label)
        (elif (<= (`/Game/Platzi/Core/Creature/BP_Tamagochibase.Health` (`self.refPet`)) 0.0)
          (set `self.battleStatus ` "NewEnumerator1")
          (else
            (set `self.battleStatus ` "NewEnumerator2")))))
    (:`else`
      (goto _label)))
  (switch `/Game/Platzi/Core/Enum/EVictory` (`self.battleStatus `)
    (:`NewEnumerator0`
      (`self.victory`))
    (:`NewEnumerator1`
      (`self.defeat`))
    (:`NewEnumerator2`
      _))
  (return))

(fn `chooseTurn`
  (bind _nextmosnter (`self.getNextParticipant`))
  (`/Engine/EditorBlueprintResources/StandardMacros.IsValid` _nextmosnter
    (:`Is Valid`
      (bind _output_get (set `self.currentMonster` _nextmosnter))
      ;[1 1 1] StarTurn
      (`/Game/Platzi/Core/Creature/BP_Tamagochibase.starTurn` _output_get))
    (:`Is Not Valid`
      (`self.getNextParticipant`))))

(fn `defeat`
  (bind _output_get (set `self.battleMessege` "Your pet has been defeated"))
  (`self.ShowMessege` _output_get)
  (`Widget.SetIsEnabled` (`/Game/Platzi/UI/WBP_Main.Button_Ability` (`/Game/Platzi/Core/Creature/Ped/BP_TamgochiPet.RefWidget` (`self.refPet`))) false)
  (`Widget.SetIsEnabled` (`/Game/Platzi/UI/WBP_Main.Button_Atack` (`/Game/Platzi/Core/Creature/Ped/BP_TamgochiPet.RefWidget` (`self.refPet`))) false)
  (`Widget.SetIsEnabled` (`/Game/Platzi/UI/WBP_Main.Button_Heal` (`/Game/Platzi/Core/Creature/Ped/BP_TamgochiPet.RefWidget` (`self.refPet`))) false)
  (`Widget.SetIsEnabled` (`/Game/Platzi/UI/WBP_Main.Button_Food` (`/Game/Platzi/Core/Creature/Ped/BP_TamgochiPet.RefWidget` (`self.refPet`))) false)
  (`Widget.SetIsEnabled` (`/Game/Platzi/UI/WBP_Main.Button_Medicine` (`/Game/Platzi/Core/Creature/Ped/BP_TamgochiPet.RefWidget` (`self.refPet`))) false)
  (`Widget.SetIsEnabled` (`/Game/Platzi/UI/WBP_Main.Button_Battle` (`/Game/Platzi/Core/Creature/Ped/BP_TamgochiPet.RefWidget` (`self.refPet`))) false)
  (`self.EndBattle`))

(fn `getNextParticipant`
  (returns (nextMosnter :type "/Game/Platzi/Core/Creature/BP_Tamagochibase Object Reference"))
  (bind _refpet (`self.refPet`))
  (`self.chechVictory`)
  (switch `int` (`self.shiftCounter`)
    (:`0`
      (set `self.shiftCounter` 1))
    (:`1`
      (set `self.shiftCounter` 0)))
  (bind _refenemy (`self.refEnemy`)
    (:`then`
      (return (select `int` (`self.shiftCounter`) :`0` _refpet :`1` _refenemy :!type "/Game/Platzi/Core/Creature/BP_Tamagochibase Object Reference")))
    (:`else`
      (return _refpet))))

(fn `loadSession`
  (bind _refsavegame (`self.refSaveGame`))
  (bind _refpet (`self.refPet`))
  (bind _returnvalue (`GameplayStatics.DoesSaveGameExist` (`self.usedSlot`)))
  (if _returnvalue
    (bind _returnvalue_2 (`GameplayStatics.LoadGameFromSlot` (`self.usedSlot`)))
    (bind _asmy_save_game (cast `/Game/Platzi/Core/mySaveGame` _returnvalue_2))
    (set `self.refSaveGame` _asmy_save_game)
    (set `/Game/Platzi/Core/Creature/BP_Tamagochibase.Health` (`/Game/Platzi/Core/mySaveGame.savedHealth` _refsavegame) _refpet)
    (set `/Game/Platzi/Core/Creature/Ped/BP_TamgochiPet.Hungry` (`/Game/Platzi/Core/mySaveGame.savedHungry` _refsavegame) _refpet)
    (set `/Game/Platzi/Core/Creature/BP_Tamagochibase.Dead` (`/Game/Platzi/Core/mySaveGame.savedDead` _refsavegame) _refpet)
    (else
      (bind _returnvalue_3 (`GameplayStatics.CreateSaveGameObject` "/Game/Platzi/Core/mySaveGame.mySaveGame_C"))
      (set `self.refSaveGame` _returnvalue_3))))

(fn `saveSession`
  (bind _refpet (`self.refPet`))
  (bind _refsavegame (`self.refSaveGame`))
  (`/Engine/EditorBlueprintResources/StandardMacros.IsValid` (`self.refSaveGame`)
    (:`Is Valid`
      _)
    (:`Is Not Valid`
      (bind _returnvalue (`GameplayStatics.CreateSaveGameObject` "/Game/Platzi/Core/mySaveGame.mySaveGame_C"))
      (set `self.refSaveGame` _returnvalue)))
  (set `/Game/Platzi/Core/mySaveGame.savedHealth` (`/Game/Platzi/Core/Creature/BP_Tamagochibase.Health` _refpet) _refsavegame)
  (set `/Game/Platzi/Core/mySaveGame.savedHungry` (`/Game/Platzi/Core/Creature/Ped/BP_TamgochiPet.Hungry` _refpet) _refsavegame)
  (set `/Game/Platzi/Core/mySaveGame.savedDead` (`/Game/Platzi/Core/Creature/BP_Tamagochibase.Dead` _refpet) _refsavegame)
  (bind _returnvalue_2 (`GameplayStatics.SaveGameToSlot` _refsavegame (`self.usedSlot`)))
  (bind _output_get (set `self.battleMessege` (`KismetTextLibrary.Conv_StringToText` (select `bool` _returnvalue_2 :`false` "Error to save" :`true` "Game Saved"))))
  (`self.ShowMessege` _output_get))

(fn `spawnEnemy`
  (bind (_returnvalue_location _returnvalue_rotation) (`KismetMathLibrary.BreakTransform` (`SceneComponent.K2_GetComponentToWorld` (`/Game/Platzi/Core/Creature/Ped/BP_TamgochiPet.EnemyLocation` (`self.refPet`)))))
  (`GameplayStatics.SpawnEmitterAtLocation` "/Game/InfinityBladeEffects/Effects/FX_Mobile/Fire/combat/P_YoYo_FireBlast_Axe_02.P_YoYo_FireBlast_Axe_02" _returnvalue_location)
  (bind _returnvalue (`|SpawnActorFromClass` "/Game/Platzi/Core/Creature/Enemy/BP_TamgochiEnemy.BP_TamgochiEnemy_C" (`KismetMathLibrary.MakeTransform` _returnvalue_location _returnvalue_rotation (3.0 3.0 3.0)) "Undefined" "OverrideRootScale" null null))
  (set `self.refEnemy` _returnvalue))

(fn `UpdateTime`
  (returns (currentTime :type "/Game/Platzi/Core/Enum/TimeOfDay Enum") (currentDay :type Integer))
  (bind _returnvalue (`KismetMathLibrary.Now`))
  (bind (_year _month _day _hour) (`KismetMathLibrary.BreakDateTime` _returnvalue))
  (set `self.currentDay` (`KismetMathLibrary.GetDayOfYear` _returnvalue))
  (if (and (>= _hour 7) (< _hour 12))
    (bind _output_get (set `self.timeDay` "NewEnumerator0"))
    (return _output_get (`self.currentDay`))
    (elif (and (>= _hour 12) (< _hour 18))
      (bind _output_get_2 (set `self.timeDay` "NewEnumerator1"))
      (return _output_get_2 (`self.currentDay`))
      (elif (and (>= _hour 18) (< _hour 23))
        (bind _output_get_3 (set `self.timeDay` "NewEnumerator1"))
        (return _output_get_3 (`self.currentDay`))
        (elif (and (>= _hour 23) (< _hour 7))
          (bind _output_get_4 (set `self.timeDay` "NewEnumerator3"))
          (return _output_get_4 (`self.currentDay`)))))))

(fn `UserConstructionScript`)

(fn `victory`
  (`self.RatateStarPosition`)
  (bind _output_get (set `self.battleMessege` "You won the battle!!"))
  (`self.ShowMessege` _output_get)
  (bind _refenemy (`self.refEnemy`)
    (:`then`
      (`/Game/Platzi/Core/Creature/Enemy/BP_TamgochiEnemy.DestroyMonster` _refenemy 1.0))
    (:`else`
      _))
  (`self.EndBattle`))