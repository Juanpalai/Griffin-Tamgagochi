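; Base creature Blueprint for turn-based pet battles, with empty attack and player-control events, apparently meant for child classes.
; StarTurn flashes a marker through a timeline-driven dynamic material on the sphere, then branches by team to player or enemy control.
; After a delay, enemies check the GameMode's pet reference and randomly attack, favoring melee over special.
; CalculateHeath applies damage to normalized health, updating Sick and a latched Dead flag.
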(event `self.ReceiveBeginPlay`)

(event `EnemyControlActions`
  (`KismetSystemLibrary.Delay` 2.0)
  (bind _asbp_my_game_mode (cast `/Game/Platzi/Core/Blueprint/BP_MyGameMode` (`GameplayStatics.GetGameMode`)))
  (`/Engine/EditorBlueprintResources/StandardMacros.IsValid` (`/Game/Platzi/Core/Blueprint/BP_MyGameMode.refPet` _asbp_my_game_mode)
    (:`Is Valid`
      (switch `int` (`KismetMathLibrary.RandomInteger` 4)
        (:`Default`
          (`self.MeleeAtack`))
        (:`0`
          (`self.SpecialAtack`))))))

(event `ShowMarker`
  (bind (_direction _opacity) (`Timeline|Flash` :!via `PlayFromStart`)
    (:`Update`
      (`MaterialInstanceDynamic.SetScalarParameterValue` (`self.refMMarker`) "Opacity" _opacity))))

(event `SpecialAtack`)

(event `MeleeAtack`)

(event `PlayerControllerActions`)

(fn `CalculateHeath`
  (params (HealthDamage :type "Float (double-precision)"))
  (bind _output_get (set `self.Health` (`KismetMathLibrary.FClamp` (- (`self.Health`) HealthDamage))))
  (set `self.Sick` (< _output_get 0.34))
  (`self.ChechDead` (`self.Dead`)))

(fn `ChechDead`
  (params (AlreadyDead :type Boolean))
  (set `self.Dead` (or (<= (`self.Health`) 0.0) AlreadyDead)))

(fn `starTurn`
  ;[1 1 1] Show Marker
  (`self.ShowMarker`)
  (if (== (`self.team`) 1)
    (`self.PlayerControllerActions`)
    (else
      (`self.EnemyControlActions`))))

(fn `UserConstructionScript`
  (bind _returnvalue (`PrimitiveComponent.CreateDynamicMaterialInstance` (`self.Sphere`) 0 "/Game/Materiales/M_marker.M_marker" "None"))
  (bind _output_get (set `self.refMMarker` _returnvalue))
  (`MaterialInstanceDynamic.SetScalarParameterValue` _output_get "Opacity" 0.0))